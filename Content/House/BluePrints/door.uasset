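; Door Blueprint for the house that swings open or shut each time its Oninteraction event fires.
; The Dooropen flag flips on each call and picks whether a timeline plays forward (when true) or reverses.
; The timeline's DoorSwing track drives the static mesh's relative yaw.
; Each interaction also adds an FMOD audio component for sound.
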(event EventOninteraction
  (if (Variables|Default|GetDooropen)
    (AddComponent|AddFMODAudioComponent false)
    (Variables|Default|SetDooropen false)
    (bind _doorswing (Timeline|Timeline_0 Play)
      (:Update
        (Transformation|SetRelativeRotation (Variables|Debug|GetStaticMeshComponent) (Math|Rotator|MakeRotator 0.0 0.0 (.Z (Math|Vector|BreakVector (Math|Vector|MakeVector _doorswing 0.0 _doorswing)))) false false)))
    (else
      (AddComponent|AddFMODAudioComponent false)
      (Variables|Default|SetDooropen true)
      (Timeline|Timeline_0 Reverse))))

(fn ConstructionScript)